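; BP_Cat is a cat pickup built from cube components that the player saves by touching it.
; On overlap with BP_ThirdPersonCharacter, it enables physics simulation on the cubes and destroys itself after a short delay.
; The same overlap immediately increments the saved cat count on BP_ThirdPersonGameMode, with no guard against repeat overlaps during the delay.
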(event `self.ReceiveActorBeginOverlap`
  (params (OtherActor :type "Actor Object Reference"))
  (cast `/Game/ThirdPerson/Blueprints/BP_ThirdPersonCharacter` OtherActor)
  (`|ExecutionSequence`
    (:`then_0`
      (`PrimitiveComponent.SetSimulatePhysics` (`self.Cube5`) true)
      (`PrimitiveComponent.SetSimulatePhysics` (`self.Cube3`) true)
      (`PrimitiveComponent.SetSimulatePhysics` (`self.Cube2`) true)
      (`PrimitiveComponent.SetSimulatePhysics` (`self.Cube1`) true)
      (`PrimitiveComponent.SetSimulatePhysics` (`self.Cube`) true)
      (`PrimitiveComponent.SetSimulatePhysics` (`self.Cube4`) true)
      (`PrimitiveComponent.SetSimulatePhysics` (`self.Cube10`) true)
      (`PrimitiveComponent.SetSimulatePhysics` (`self.Cube9`) true)
      (`PrimitiveComponent.SetSimulatePhysics` (`self.Cube8`) true)
      (`PrimitiveComponent.SetSimulatePhysics` (`self.Cube7`) true)
      (`PrimitiveComponent.SetSimulatePhysics` (`self.Cube6`) true)
      (`KismetSystemLibrary.Delay` 3.0)
      (`self.K2_DestroyActor`))
    (:`then_1`
      (`/Game/ThirdPerson/Blueprints/BP_ThirdPersonGameMode.IncrementSavedCat` (cast `/Game/ThirdPerson/Blueprints/BP_ThirdPersonGameMode` (`GameplayStatics.GetGameMode`) :!pure true)))))

(fn `UserConstructionScript`)