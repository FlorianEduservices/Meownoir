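; BP_DynamiqueSpikes is a spike trap that starts lowered and springs up when a BP_ThirdPersonCharacter overlaps it.
; A timeline drives the Z offset of the Scene component to raise the spikes.
; At the top, it damages every actor still overlapping the trap, whatever its class, then reverses the timeline to retract.
; The end-overlap event only casts and triggers nothing.
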(event `self.ReceiveBeginPlay`
  (`SceneComponent.K2_SetRelativeLocation` (`self.Scene`) (0.0 0.0 -60.0) false false))

(event `self.ReceiveActorBeginOverlap`
  (params (OtherActor :type "Actor Object Reference"))
  (cast `/Game/ThirdPerson/Blueprints/BP_ThirdPersonCharacter` OtherActor)
  (bind (_direction _location) (`Timeline|Timeline` :!label _label)
    (:`Update`
      (`SceneComponent.K2_SetRelativeLocation` (`self.Scene`) (`KismetMathLibrary.MakeVector` 0.0 0.0 (`KismetMathLibrary.Lerp` -60.0 60.0 _location)) false false))
    (:`Finished`
      (if (`|EnumEquality` _direction "Forward")
        (`|ExecutionSequence`
          (:`then_0`
            (for _array_element (`self.GetOverlappingActors` null)
              (`GameplayStatics.ApplyDamage` _array_element 1.0)))
          (:`then_1`
            (goto _label :!via `ReverseFromEnd`)))))))

(event `self.ReceiveActorEndOverlap`
  (params (OtherActor :type "Actor Object Reference"))
  (cast `/Game/ThirdPerson/Blueprints/BP_ThirdPersonCharacter` OtherActor))

(fn `UserConstructionScript`)