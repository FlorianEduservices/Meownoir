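; BP_MovingPlateform is a moving platform that shuttles back and forth along its relative X axis.
; On BeginPlay, it waits for a configurable start delay, then sets the timeline play rate from TimeRate.
; A FlipFlop alternates the timeline between forward and reverse, re-triggered on each finish for an endless ping-pong.
; The timeline's Movement track, scaled by TravelLength, drives the platform's location.
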(event `self.ReceiveBeginPlay`
  (`KismetSystemLibrary.Delay` (`self.DurationBeforeStart`))
  (`TimelineComponent.SetPlayRate` (`self.MovementTimeline`) (`self.TimeRate`))
  (`/Engine/EditorBlueprintResources/StandardMacros.FlipFlop` :!label _label
    (:`A`
      (bind (_direction _movement) (`Timeline|MovementTimeline` :!via `PlayFromStart` :!label _label_2)
        (:`Update`
          (`SceneComponent.K2_SetRelativeLocation` (`self.Plateform`) (`KismetMathLibrary.MakeVector` (* _movement (`self.TravelLength`))) false false))
        (:`Finished`
          (goto _label))))
    (:`B`
      (goto _label_2 :!via `ReverseFromEnd`))))

(event `self.ReceiveTick`
  (params (DeltaSeconds :type "Float (single-precision)")))

(fn `UserConstructionScript`)